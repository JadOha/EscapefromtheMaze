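; BP_TargetAI is a shootable AI target that adds one point to the first-person player character's score when destroyed.
; Hit events on head, body and arm components respond to BP_FirstPersonProjectile, with headshots dealing double damage and setting a Headshot flag.
; Tick feeds health into a widget-component health bar, turns it toward the player camera, and destroys the actor once health reaches zero.
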(event `self.ReceiveTick`
  (params (DeltaSeconds :type "Float (single-precision)"))
  (bind _healthbarwidget (`self.HealthBarWidget`))
  ;[1 1 1] Score Counter
  (bind _aswb_aihealth_bar (cast `/Game/HUDs/WB_AIHealthBar` (`WidgetComponent.GetWidget` (`self.HealthBarWidget`))))
  (`ProgressBar.SetPercent` (`/Game/HUDs/WB_AIHealthBar.HealthBar` _aswb_aihealth_bar) (/ (`self.AIHealth`) 100.0))
  (`SceneComponent.K2_SetWorldRotation` _healthbarwidget (`KismetMathLibrary.FindLookAtRotation` (`SceneComponent.K2_GetComponentLocation` _healthbarwidget) (`SceneComponent.K2_GetComponentLocation` (`PlayerCameraManager.TransformComponent` (`GameplayStatics.GetPlayerCameraManager` 0)))) false false)
  (if (<= (`self.AIHealth`) 0.0)
    (`self.K2_DestroyActor`)))

(event `self.Body.OnComponentHit`
  (params (HitComponent :type "PrimitiveComponent Object Reference") (OtherActor :type "Actor Object Reference") (OtherComp :type "PrimitiveComponent Object Reference") (NormalImpulse :type "Vector Structure") (Hit :type "HitResult Structure (by ref)"))
  ;[1 1 1] Projectile collision w/ body check
  (cast `/Game/FirstPerson/Blueprints/BP_FirstPersonProjectile` OtherActor)
  (cast `/Game/FirstPerson/Blueprints/BP_FirstPersonGameMode` (`GameplayStatics.GetGameMode`))
  (if true
    (`KismetSystemLibrary.PrintString` "Body Shot")
    (set `self.headshot?` false)
    (set `self.AIHealth` (- (`self.AIHealth`) 15.0))))

(event `self.Arm.OnComponentHit`
  (params (HitComponent :type "PrimitiveComponent Object Reference") (OtherActor :type "Actor Object Reference") (OtherComp :type "PrimitiveComponent Object Reference") (NormalImpulse :type "Vector Structure") (Hit :type "HitResult Structure (by ref)"))
  ;[1 1 1] Projectile collision w/ arm check
  (cast `/Game/FirstPerson/Blueprints/BP_FirstPersonProjectile` OtherActor)
  (cast `/Game/FirstPerson/Blueprints/BP_FirstPersonGameMode` (`GameplayStatics.GetGameMode`))
  (if true
    (`KismetSystemLibrary.PrintString` "Body Shot")
    (set `self.headshot?` false)
    (set `self.AIHealth` (- (`self.AIHealth`) 15.0))))

(event `self.Head.OnComponentHit`
  (params (HitComponent :type "PrimitiveComponent Object Reference") (OtherActor :type "Actor Object Reference") (OtherComp :type "PrimitiveComponent Object Reference") (NormalImpulse :type "Vector Structure") (Hit :type "HitResult Structure (by ref)"))
  ;[1 1 1] Projectile collision w/ head check
  (cast `/Game/FirstPerson/Blueprints/BP_FirstPersonProjectile` OtherActor)
  (`KismetSystemLibrary.PrintString` "Headshot")
  (set `self.headshot?` true)
  (set `self.AIHealth` (- (`self.AIHealth`) 30.0)))

(event `self.ReceiveDestroyed`
  (bind _asbp_first_person_character (cast `/Game/FirstPerson/Blueprints/BP_FirstPersonCharacter` (`GameplayStatics.GetPlayerCharacter` 0)))
  (bind _result (`/Engine/EditorBlueprintResources/StandardMacros.IncrementInt` (`/Game/FirstPerson/Blueprints/BP_FirstPersonCharacter.Score` _asbp_first_person_character))
    (:`  `
      (set `/Game/FirstPerson/Blueprints/BP_FirstPersonCharacter.Score` _result _asbp_first_person_character))))

(fn `UserConstructionScript`)